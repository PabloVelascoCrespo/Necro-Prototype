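; BP_Grid is the grid actor that builds the cell map and relays move commands to the minions and enemies on it.
; On BeginPlay, Init spawns BP_GridCell actors row by row into GridCellArray, then the player pawn teleports to the first cell after a short delay.
; Entities register in GridArray through AddEnitity, and separate move events cast each entry to BP_Minion or BP_Enemy to call CEMove.
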(event Custom|AddEnitity
  (params (NewEntity :type BP%20Generic%20Entity%20Object%20Reference))
  (Utilities|Array|Add (Variables|Default|GetGridArray) NewEntity))

(event Custom|CE_MoveMinions
  (for _array_element (Variables|Default|GetGridArray)
    (bind _asbp_minion (Utilities|Casting|CastToBP_Minion _array_element))
    (Default|CEMove _asbp_minion)
    (Development|PrintString (Utilities|String|ToString(Integer) (Variables|/Game/Blueprints/Characters/BP_GenericEntity.BP_GenericEntity_C|GetGridPosition _asbp_minion)))))

(event Custom|CE_MoveEnemies
  (for _array_element (Variables|Default|GetGridArray)
    (bind _asbp_enemy (Utilities|Casting|CastToBP_Enemy _array_element))
    (Default|CEMove _asbp_enemy)))

(event EventBeginPlay
  (CallFunction|Init)
  (Utilities|FlowControl|Delay 1.0)
  (bind _pos (Default|GetActorGridLocation (Utilities|Array|Get(acopy) (Variables|Default|GetGridCellArray))))
  (Transformation|SetActorLocation (Game|Player|GetPlayerPawn 0) _pos false false))

(fn ConstructionScript)

(fn Init
  (bind _gridcellsize (Variables|Default|GetGridCellSize))
  (bind _gridcellsize_2 (Variables|Default|GetGridCellSize))
  (while (LocalVariables|GetCompleted)
    (bind _returnvalue (Game|SpawnActorfromClass "/Game/Blueprints/BP_GridCell.BP_GridCell_C" (Math|Transform|MakeTransform (LocalVariables|GetCurrentSpawn) "0, 0, 0" "1.000000,1.000000,1.000000") "Undefined" "MultiplyWithRoot" 0 0))
    (Utilities|Array|Add (Variables|Default|GetGridCellArray) _returnvalue)
    (if (> (.X (Math|Vector|BreakVector (+ (LocalVariables|GetCurrentSpawn) (Math|Vector|MakeVector (.x _gridcellsize) 0.0 0.0)))) (* (Variables|Default|GetGridWidth) (.x _gridcellsize)))
      (LocalVariables|SetCurrentSpawn (+ (LocalVariables|GetCurrentSpawn) (Math|Vector|MakeVector (- 0.0 (.X (Math|Vector|BreakVector (LocalVariables|GetCurrentSpawn)))) (.y (Variables|Default|GetGridCellSize)) 0.0)))
      (if (> (.Y (Math|Vector|BreakVector (+ (LocalVariables|GetCurrentSpawn) (Math|Vector|MakeVector 0.0 (.y _gridcellsize_2) 0.0)))) (* (Variables|Default|GetGridHeigth) (.y _gridcellsize_2)))
        (LocalVariables|SetCompleted false))
      (else
        (LocalVariables|SetCurrentSpawn (+ (LocalVariables|GetCurrentSpawn) (Math|Vector|MakeVector (.x (Variables|Default|GetGridCellSize)) 0.0 0.0)))))))