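; Base zombie Blueprint for grid-based movement and attacks on linked cells.
; CEMove clears the current cell's Entity, teleports to the neighbor in MoveDirection and updates ActualCell, without setting the new cell's Entity here.
; CE_Atack calls CEDamage on any valid Entity in that neighboring cell.
; PrincipalLogic repeats moves in a loop governed by the Movement counter, then triggers the attack.
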(event Custom|CE_Atack
  (switch Utilities|FlowControl|Switch|SwitchonE_MoveDirection (Variables|Default|GetMoveDirection)
    (:NewEnumerator0
      (Utilities|IsValid (Variables|/Game/Blueprints/BP_GridCell.BP_GridCell_C|GetEntity (Variables|/Game/Blueprints/BP_GridCell.BP_GridCell_C|GetTopCell (Variables|Default|GetActualCell)))
        (:Is%20Valid
          (Default|CEDamage (Variables|/Game/Blueprints/BP_GridCell.BP_GridCell_C|GetEntity (Variables|/Game/Blueprints/BP_GridCell.BP_GridCell_C|GetTopCell (Variables|Default|GetActualCell)))))))
    (:NewEnumerator1
      (Utilities|IsValid (Variables|/Game/Blueprints/BP_GridCell.BP_GridCell_C|GetEntity (Variables|/Game/Blueprints/BP_GridCell.BP_GridCell_C|GetBottomCell (Variables|Default|GetActualCell)))
        (:Is%20Valid
          (Default|CEDamage (Variables|/Game/Blueprints/BP_GridCell.BP_GridCell_C|GetEntity (Variables|/Game/Blueprints/BP_GridCell.BP_GridCell_C|GetBottomCell (Variables|Default|GetActualCell)))))))
    (:NewEnumerator2
      (Utilities|IsValid (Variables|/Game/Blueprints/BP_GridCell.BP_GridCell_C|GetEntity (Variables|/Game/Blueprints/BP_GridCell.BP_GridCell_C|GetRightCell (Variables|Default|GetActualCell)))
        (:Is%20Valid
          (Default|CEDamage (Variables|/Game/Blueprints/BP_GridCell.BP_GridCell_C|GetEntity (Variables|/Game/Blueprints/BP_GridCell.BP_GridCell_C|GetRightCell (Variables|Default|GetActualCell)))))))
    (:NewEnumerator3
      (Utilities|IsValid (Variables|/Game/Blueprints/BP_GridCell.BP_GridCell_C|GetEntity (Variables|/Game/Blueprints/BP_GridCell.BP_GridCell_C|GetLeftCell (Variables|Default|GetActualCell)))
        (:Is%20Valid
          (Default|CEDamage (Variables|/Game/Blueprints/BP_GridCell.BP_GridCell_C|GetEntity (Variables|/Game/Blueprints/BP_GridCell.BP_GridCell_C|GetLeftCell (Variables|Default|GetActualCell)))))))))

(event EventCEMove
  (Variables|/Game/Blueprints/BP_GridCell.BP_GridCell_C|SetEntity (Variables|Default|GetActualCell) 0)
  (switch Utilities|FlowControl|Switch|SwitchonE_MoveDirection (Variables|Default|GetMoveDirection)
    (:NewEnumerator0
      (bind _pos (Default|GetActorGridLocation (Variables|/Game/Blueprints/BP_GridCell.BP_GridCell_C|GetTopCell (Variables|Default|GetActualCell)) self))
      (Transformation|SetActorLocation _pos false false)
      (Variables|Default|SetActualCell (Variables|/Game/Blueprints/BP_GridCell.BP_GridCell_C|GetTopCell (Variables|Default|GetActualCell)))
      (Utilities|FlowControl|Delay 0.5))
    (:NewEnumerator1
      (bind _pos_2 (Default|GetActorGridLocation (Variables|/Game/Blueprints/BP_GridCell.BP_GridCell_C|GetBottomCell (Variables|Default|GetActualCell)) self))
      (Transformation|SetActorLocation _pos_2 false false)
      (Variables|Default|SetActualCell (Variables|/Game/Blueprints/BP_GridCell.BP_GridCell_C|GetBottomCell (Variables|Default|GetActualCell)))
      (Utilities|FlowControl|Delay 0.5))
    (:NewEnumerator2
      (bind _pos_3 (Default|GetActorGridLocation (Variables|/Game/Blueprints/BP_GridCell.BP_GridCell_C|GetRightCell (Variables|Default|GetActualCell)) self))
      (Transformation|SetActorLocation _pos_3 false false)
      (Variables|Default|SetActualCell (Variables|/Game/Blueprints/BP_GridCell.BP_GridCell_C|GetRightCell (Variables|Default|GetActualCell)))
      (Utilities|FlowControl|Delay 0.5))
    (:NewEnumerator3
      (bind _pos_4 (Default|GetActorGridLocation (Variables|/Game/Blueprints/BP_GridCell.BP_GridCell_C|GetLeftCell (Variables|Default|GetActualCell)) self))
      (Transformation|SetActorLocation _pos_4 false false)
      (Variables|Default|SetActualCell (Variables|/Game/Blueprints/BP_GridCell.BP_GridCell_C|GetLeftCell (Variables|Default|GetActualCell)))
      (Utilities|FlowControl|Delay 0.5))))

(fn ConstructionScript
  (|CallParentFunction))

(fn PrincipalLogic
  (while (> (Variables|Default|GetMovement) (LocalVariables|Geti))
    (CallFunction|CEMove)
    (Math|Integer|IncrementInt (Variables|Default|GetMovement)))
  (CallFunction|CEAtack))