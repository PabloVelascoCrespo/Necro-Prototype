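; Player pawn for a grid-based game, with mouse-driven movement and a rotatable spring-arm camera.
; BeginPlay shows the mouse cursor, and Q and E rotate the spring arm in yaw steps by RotationVelocity.
; Right-click traces from the cursor on the Visibility channel, and a hit BP_GridCell supplies its grid location to MoveToPos.
; MoveToPos teleports the actor there instantly without sweep, pathfinding or interpolation.
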(event Custom|MoveToPos
  (params (Pos :type Vector))
  (Transformation|SetActorLocation Pos false false))

(event EventBeginPlay
  ;[1 1 1] Beguin
  (Variables|/Script/Engine.PlayerController|SetbShowMouseCursor (Game|GetPlayerController 0) true))

(event Input|KeyboardEvents|E
  (params (Key :type Key%20Structure :default "None"))
  ;[1 1 1] Movimieto de camara
  (:Pressed
    (Transformation|AddLocalRotation (Variables|Default|GetSpringArm) (Math|Rotator|MakeRotator 0.0 0.0 (- 0.0 (Variables|Default|GetRotationVelocity))) false false)))

(event Input|KeyboardEvents|Q
  (params (Key :type Key%20Structure :default "None"))
  ;[1 1 1] Movimieto de camara
  (:Pressed
    (Transformation|AddLocalRotation (Variables|Default|GetSpringArm) (Math|Rotator|MakeRotator 0.0 0.0 (Variables|Default|GetRotationVelocity)) false false)))

(event Input|MouseEvents|RightMouseButton
  (params (Key :type Key%20Structure :default "None"))
  (bind _returnvalue (Game|GetPlayerController 0))
  (bind (_worldlocation _worlddirection) (Game|Player|ConvertMouseLocationToWorldSpace _returnvalue))
  ;[1 1 1] Rayo para moverte
  (:Pressed
    (bind (_outhit _returnvalue_2) (Collision|LineTraceByChannel _worldlocation (+ _worldlocation (* _worlddirection (Math|Conversions|ToVector(Float) 1e+04))) "TraceTypeQuery1" false 0 "None"))
    (if _returnvalue_2
      (bind _asbp_grid_cell (Utilities|Casting|CastToBP_GridCell (.HitActor (Collision|BreakHitResult _outhit))))
      (bind _pos (Default|GetActorGridLocation _asbp_grid_cell))
      (CallFunction|MovetoPos _pos))))

(fn ConstructionScript)