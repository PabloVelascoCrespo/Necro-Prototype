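; BP_GenericEntity is a generic character entity with life, death and position-swap events, plus empty attack and MainLogic stubs.
; CE_Damage decrements Life by one, prints it and calls the death event at zero or below, which destroys the actor; a trailing Delay leads to nothing.
; CE_ChangePositions swaps locations with another entity without sweep or teleport, storing the other's location in AuxLocation first.
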(event Custom|CE_Damage
  (bind _result (Math|Integer|DecrementInt (Variables|Default|GetLife))
    (:%20%20
      (Development|PrintString (Utilities|String|ToString(Integer) _result))
      (if (<= _result 0)
        (CallFunction|CEDie))
      (Utilities|FlowControl|Delay 0.4))))

(event Custom|CE_Atack)

(event Custom|CE_ChangePositions
  (params (OtherGE :type BP%20Generic%20Entity%20Object%20Reference))
  (Variables|Default|SetAuxLocation (Transformation|GetActorLocation OtherGE))
  (Transformation|SetActorLocation (Transformation|GetActorLocation OtherGE) false false)
  (Transformation|SetActorLocation OtherGE (Variables|Default|GetAuxLocation) false false))

(event Custom|CE_Die
  (Actor|DestroyActor))

(fn ConstructionScript)

(fn MainLogic)