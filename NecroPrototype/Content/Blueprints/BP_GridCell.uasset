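; Grid cell actor that toggles its validity and floor material between available and blocked, apparently to show movement range.
; Activation events cascade through the Right, Left, Top and Bottom cell references, spreading up to three steps outward.
; CE_Ice applies the frozen material to the surrounding 3x3 block without null checks or changing validity.
; GetActorGridLocation returns the actor location plus an offset.
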(event Custom|Block%20Self
  (Variables|Default|SetIsValid false)
  (Rendering|Material|SetMaterial (Variables|Default|Getsuelo) 0 "/Game/Materials/Cell_instancce_Block.Cell_instancce_Block"))

(event Custom|Activate%203%20layer
  (Variables|Default|SetIsValid true)
  (Rendering|Material|SetMaterial (Variables|Default|Getsuelo) 0 "/Game/Materials/Cell_instancce_Aviable.Cell_instancce_Aviable")
  (Utilities|FlowControl|Sequence
    (:then_0
      (if (Utilities|IsValid (Variables|Default|GetRightCell))
        (CallFunction|Activate2Layer (Variables|Default|GetRightCell))))
    (:then_1
      (if (Utilities|IsValid (Variables|Default|GetLeftCell))
        (CallFunction|Activate2Layer (Variables|Default|GetLeftCell))))
    (:then_2
      (if (Utilities|IsValid (Variables|Default|GetTopCell))
        (CallFunction|Activate2Layer (Variables|Default|GetTopCell))))
    (:then_3
      (if (Utilities|IsValid (Variables|Default|GetBottomCell))
        (CallFunction|Activate2Layer (Variables|Default|GetBottomCell))))))

(event Custom|Activate%20Self
  (Variables|Default|SetIsValid true)
  (Rendering|Material|SetMaterial (Variables|Default|Getsuelo) 0 "/Game/Materials/Cell_instancce_Aviable.Cell_instancce_Aviable"))

(event Custom|CE_Ice
  ;[1 1 1] CONGELAR EL SUELO (al subir el número de casillas que se puede mover se cambia de nuevo a rojo)
  (Rendering|Material|SetMaterial (Variables|Default|Getsuelo) 0 "/Game/Materials/Cell_instance_Frozen.Cell_instance_Frozen")
  (Rendering|Material|SetMaterial (Variables|BP_GridCell_C|Getsuelo (Variables|Default|GetRightCell)) 0 "/Game/Materials/Cell_instance_Frozen.Cell_instance_Frozen")
  (Rendering|Material|SetMaterial (Variables|BP_GridCell_C|Getsuelo (Variables|Default|GetLeftCell)) 0 "/Game/Materials/Cell_instance_Frozen.Cell_instance_Frozen")
  (Rendering|Material|SetMaterial (Variables|BP_GridCell_C|Getsuelo (Variables|Default|GetTopCell)) 0 "/Game/Materials/Cell_instance_Frozen.Cell_instance_Frozen")
  (Rendering|Material|SetMaterial (Variables|BP_GridCell_C|Getsuelo (Variables|Default|GetBottomCell)) 0 "/Game/Materials/Cell_instance_Frozen.Cell_instance_Frozen")
  (Rendering|Material|SetMaterial (Variables|BP_GridCell_C|Getsuelo (Variables|BP_GridCell_C|GetLeftCell (Variables|Default|GetTopCell))) 0 "/Game/Materials/Cell_instance_Frozen.Cell_instance_Frozen")
  (Rendering|Material|SetMaterial (Variables|BP_GridCell_C|Getsuelo (Variables|BP_GridCell_C|GetRightCell (Variables|Default|GetTopCell))) 0 "/Game/Materials/Cell_instance_Frozen.Cell_instance_Frozen")
  (Rendering|Material|SetMaterial (Variables|BP_GridCell_C|Getsuelo (Variables|BP_GridCell_C|GetRightCell (Variables|Default|GetBottomCell))) 0 "/Game/Materials/Cell_instance_Frozen.Cell_instance_Frozen")
  (Rendering|Material|SetMaterial (Variables|BP_GridCell_C|Getsuelo (Variables|BP_GridCell_C|GetLeftCell (Variables|Default|GetBottomCell))) 0 "/Game/Materials/Cell_instance_Frozen.Cell_instance_Frozen"))

(event Custom|ActiveConnecteds
  (Variables|Default|SetIsValid true)
  (Rendering|Material|SetMaterial (Variables|Default|Getsuelo) 0 "/Game/Materials/Cell_instancce_Aviable.Cell_instancce_Aviable")
  (Utilities|FlowControl|Sequence
    (:then_0
      (if (Utilities|IsValid (Variables|Default|GetRightCell))
        (CallFunction|ActivateSelf (Variables|Default|GetRightCell))))
    (:then_1
      (if (Utilities|IsValid (Variables|Default|GetLeftCell))
        (CallFunction|ActivateSelf (Variables|Default|GetLeftCell))))
    (:then_2
      (if (Utilities|IsValid (Variables|Default|GetTopCell))
        (CallFunction|ActivateSelf (Variables|Default|GetTopCell))))
    (:then_3
      (if (Utilities|IsValid (Variables|Default|GetBottomCell))
        (CallFunction|ActivateSelf (Variables|Default|GetBottomCell))))))

(event Custom|Activate%202%20layer
  (Variables|Default|SetIsValid true)
  (Rendering|Material|SetMaterial (Variables|Default|Getsuelo) 0 "/Game/Materials/Cell_instancce_Aviable.Cell_instancce_Aviable")
  (Utilities|FlowControl|Sequence
    (:then_0
      (if (Utilities|IsValid (Variables|Default|GetRightCell))
        (CallFunction|ActiveConnecteds (Variables|Default|GetRightCell))))
    (:then_1
      (if (Utilities|IsValid (Variables|Default|GetLeftCell))
        (CallFunction|ActiveConnecteds (Variables|Default|GetLeftCell))))
    (:then_2
      (if (Utilities|IsValid (Variables|Default|GetTopCell))
        (CallFunction|ActiveConnecteds (Variables|Default|GetTopCell))))
    (:then_3
      (if (Utilities|IsValid (Variables|Default|GetBottomCell))
        (CallFunction|ActiveConnecteds (Variables|Default|GetBottomCell))))))

(fn ConstructionScript)

(fn GetActorGridLocation
  (return (+ (Variables|Default|GetOffset) (Transformation|GetActorLocation))))